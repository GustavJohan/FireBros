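; Game instance for Firebros that handles hosting and joining multiplayer sessions through Advanced Sessions nodes, with a LAN toggle.
; Hosting creates a session and opens the Lobby level as a listen server.
; Joining searches again, matches the selected session by ID string, then joins it, printing debug messages along the way.
; Both flows show a loading screen on the multiplayer menu widget and hide it on failure.
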(event Custom|Host%20Session
  (CallFunction|ToggleLoadignScreen true)
  (|AdvancedSession 0 (Game|GetPlayerController 0) 100 0 (Variables|Default|GetLan) true false true true true false false false true false true
    (:OnSuccess
      (Game|OpenLevel(byObjectReference) "/Game/Levels/Lobby.Lobby" true "listen"))
    (:OnFailure
      (CallFunction|ToggleLoadignScreen false))))

(event Custom|Join%20Session
  (params (Selected%20session :type Blueprint%20Session%20Result%20Structure))
  (bind _returnvalue (Game|GetPlayerController 0))
  (CallFunction|ToggleLoadignScreen true)
  (Development|PrintString "begin join")
  (bind _results (|FindSessionsAdvanced _returnvalue 100 (Variables|Default|GetLan) "AllServers" 0 false false false true)
    (:OnSuccess
      (bind _array_element (Utilities|Array|ForEachLoopwithBreak _results :!label _label)
        (:LoopBody
          (if (Utilities|Enum|Equal(Enum) (Class|AdvancedSessionsLibrary|GetSessionIDasString Selected%20session) (Class|AdvancedSessionsLibrary|GetSessionIDasString _array_element))
            (Development|PrintString "found")
            (goto _label Break)
            (else
              (Development|PrintString "not found"))))
        (:Completed
          (|JoinSession _returnvalue _array_element
            (:OnSuccess
              (Development|PrintString "joined"))
            (:OnFailure
              (Development|PrintString "failed to join, why? has i ever?")
              (CallFunction|ToggleLoadignScreen false))))))
    (:OnFailure
      (Development|PrintString "find session failed")
      (CallFunction|ToggleLoadignScreen false))))

(fn ToggleLoadignScreen
  (params (Enable :type Boolean))
  (bind _foundwidgets (Widget|GetAllWidgetsOfClass "/Game/Blueprints/Widgets/MultiplayerMenuWidget_WBP.MultiplayerMenuWidget_WBP_C" true))
  (Default|ToggleLoadingScreen (Utilities|Array|Get(acopy) _foundwidgets) Enable))