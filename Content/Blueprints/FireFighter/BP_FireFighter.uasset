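; Networked player firefighter character that carries objects and tools, can ragdoll, and shows health on a HUD.
; BeginPlay applies physical animation to bodies below a named bone and creates the local player's HUD, refreshed by health replication events.
; Pickups attach to an anchor or right-hand socket, and object drops detach through a server-to-multicast RPC chain.
; R requests ragdoll through a server event, while ragdoll pickup and throw events toggle movement.
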(event Custom|Begin%20RagdollToServer
  (Class|RagdollCharacter|BeginRagdoll 5.0))

(event Custom|Pick%20Up%20Tool%20RPC
  (params (PickedUpActor :type Actor%20Object%20Reference))
  (Transformation|AttachComponentToComponent PickedUpActor (Variables|Character|GetMesh) "hand_rSocket" "SnapToTarget" "SnapToTarget" "KeepWorld" true)
  (Development|PrintString "Hello"))

(event Custom|Hit%20Obj%20Event%20Server%20RPC
  (Development|PrintString "Hit object event"))

(event Custom|DiscardObjectMulticast
  (params (NewParam :type Actor%20Object%20Reference))
  (Development|PrintString (Utilities|GetDisplayName NewParam))
  (Transformation|DetachFromActor NewParam "KeepWorld" "KeepWorld" "KeepWorld"))

(event Custom|DiscardObjectToServer
  (params (NewParam :type Actor%20Object%20Reference))
  (Development|PrintString (Utilities|GetDisplayName NewParam))
  (CallFunction|DiscardObjectMulticast NewParam))

(event EventBeginPlay
  (CallFunction|SetPhysicsAnimation)
  (Input|SetInputModeGameOnly (Game|GetPlayerController 0) false)
  (if (Pawn|IsLocallyControlled)
    (bind _returnvalue (UserInterface|CreateWidget "/Game/Blueprints/Widgets/PlayerHUD_WBP.PlayerHUD_WBP_C" (Game|GetPlayerController 0)))
    (bind _output_get (Variables|Default|SetPlayerHud _returnvalue))
    (UserInterface|Viewport|AddtoViewport _output_get 0)
    (Default|UpdateHealth (Variables|Default|GetPlayerHud) (/ (Variables|Default|GetHealth) 1e+02))))

(event EventHitObj
  (CallFunction|HitObjEventServerRPC))

(event EventDiscardTool
  (params (Discarded :type Actor%20Object%20Reference))
  (Transformation|DetachFromActor Discarded "KeepWorld" "KeepWorld" "KeepWorld"))

(event EventPickUpObject
  (params (PickedUp :type Actor%20Object%20Reference))
  (Transformation|AttachComponentToComponent PickedUp (Variables|Default|Get_PickedUpObjAnchor) "None" "SnapToTarget" "SnapToTarget" "KeepWorld" true))

(event EventPickUpTool
  (params (PickedUp :type Actor%20Object%20Reference))
  (CallFunction|PickUpToolRPC PickedUp))

(event EventDiscardObject
  (params (Discarded :type Actor%20Object%20Reference))
  (Development|PrintString (Utilities|GetDisplayName Discarded))
  (CallFunction|DiscardObjecttoServer Discarded))

(event EventRagdollPickupEvent
  (Pawn|Components|CharacterMovement|DisableMovement (Variables|Character|GetCharacterMovement)))

(event EventRagdollThrowEvent
  (Pawn|Components|CharacterMovement|SetMovementMode (Variables|Character|GetCharacterMovement) "MOVE_Walking" 0))

(event EventRepHealthtoBlueprint
  (if (Pawn|IsLocallyControlled)
    (Default|UpdateHealth (Variables|Default|GetPlayerHud) (/ (Variables|Default|GetHealth) 1e+02))))

(event Input|KeyboardEvents|R
  (params (Key :type Key%20Structure :default "None"))
  (:Pressed
    (if (Pawn|IsLocallyControlled)
      (CallFunction|BeginRagdolltoServer))))

(fn ConstructionScript)

(fn SetPhysicsAnimation
  (bind _physicalanimation (Variables|Default|GetPhysicalAnimation))
  (bind _body_name (Variables|Default|GetBody%20Name))
  (Class|PhysicalAnimationComponent|SetSkeletalMeshComponent _physicalanimation (Variables|Character|GetMesh))
  (Class|PhysicalAnimationComponent|ApplyPhysicalAnimationSettingsBelow _physicalanimation _body_name (Utilities|Struct|MakePhysicalAnimationData true 1e+03 1e+02 1e+03 1e+02) true)
  (Class|SkeletalMeshComponent|SetAllBodiesBelowSimulatePhysics (Variables|Character|GetMesh) _body_name true false))