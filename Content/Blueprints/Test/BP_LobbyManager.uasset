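; Lobby manager Blueprint that shows player names on lobby mannequins.
; SetPlayerName calls SetLocalName on the player's controller, then looks up that player's mannequin in PlayerManequins and appends it to an array.
; Setnewname stores a name, waits briefly, then pairs mannequins and names by array index, passing each to SetNameMulticast.
; That loop also removes invalid mannequins and their names from both arrays while iterating.
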(event Custom|SetNameMulticast
  (params (Mannequin :type BP%20Lobby%20Manequin%20Object%20Reference) (Name :type Text))
  (Default|SetName Mannequin Name))

(event Custom|Set%20new%20name
  (params (Name :type Text))
  (bind _mannequin (Variables|Default|GetMannequin))
  (bind _names (Variables|Default|GetNames))
  (Utilities|Array|Add (Variables|Default|GetNames) Name)
  (Utilities|FlowControl|Delay 0.5)
  (for (_array_element _array_index) _mannequin
    (if (Utilities|IsValid _array_element)
      (CallFunction|SetNameMulticast _array_element (Utilities|Array|Get(acopy) _names _array_index))
      (else
        (Utilities|Array|RemoveIndex _mannequin _array_index)
        (Utilities|Array|RemoveIndex _names _array_index)))))

(event EventSetPlayerName
  (params (relevantPlayer :type Controller%20Object%20Reference))
  (bind _playermanequins (Variables|Default|GetPlayerManequins))
  (bind (_value _returnvalue) (Utilities|Map|Find _playermanequins relevantPlayer))
  (bind _asbp_player_controller (Utilities|Casting|CastToBP_PlayerController relevantPlayer))
  (Default|SetLocalName _asbp_player_controller)
  (if _returnvalue
    (bind _asbp_lobby_manequin (Utilities|Casting|CastToBP_LobbyManequin (.MannequinActor (Utilities|Struct|BreakPlayerMannequinInformation _value))))
    (Utilities|Array|Add (Variables|Default|GetMannequin) _asbp_lobby_manequin)))

(fn ConstructionScript)