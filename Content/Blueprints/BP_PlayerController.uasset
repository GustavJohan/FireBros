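; Player controller for the firefighter game that handles join timing and passes the player's name to the pawn.
; BeginPlay sets game-only input, polls with short delays until a pawn exists, then notifies BP_GameManager of the join so UI stays in sync.
; SetLocalName reads the name from the game instance and forwards it through SetNewNameToServer to BP_FireFighter.
; ClearViewport removes all widgets, while AddClientLobbywidget is an empty stub.
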(event Custom|Add%20Client%20Lobby%20widget)

(event Custom|Set%20Local%20Name
  (Development|PrintString "setting local name" true true "(R=0.000000,G=0.247500,B=0.375000,A=1.000000)" 3.0)
  (bind _local_player_name (CallFunction|GetLocalName))
  (Development|PrintText _local_player_name)
  (bind _output_get (Variables|Default|SetPlayerName _local_player_name))
  (CallFunction|SetNewNametoServer _output_get))

(event Custom|Set%20new%20name%20to%20server
  (params (Name :type Text))
  (bind _asbp_fire_fighter (Utilities|Casting|CastToBP_FireFighter (Pawn|GetControlledPawn)))
  (Default|SetPlayerName _asbp_fire_fighter Name))

(event Custom|Clear%20Viewport
  (Viewport|RemoveAllWidgets))

(event EventBeginPlay
  (Input|SetInputModeGameOnly self false)
  ;[1 1 1] This is to ensure proper syncronization of the UI, the local player character must excist and a slight extra delay is needed to ensure that that the character is setup
  (Utilities|IsValid (Pawn|GetControlledPawn) :!label _label
    (:Is%20Valid
      (bind _returnvalue (Actor|GetActorOfClass "/Game/Blueprints/BP_GameManager.BP_GameManager_C"))
      (Utilities|FlowControl|Delay 0.2)
      (Utilities|IsValid _returnvalue
        (:Is%20Valid
          (Default|PlayerJoinEvent _returnvalue))))
    (:Is%20Not%20Valid
      (Utilities|FlowControl|Delay 0.2)
      (goto _label))))

(event EventTick
  (params (DeltaSeconds :type Float%20%28single-precision%29)))

(fn ConstructionScript)

(fn GetLocalName
  (bind _asfirebros_game_instance_bp (Utilities|Casting|CastToFirebrosGameInstance_BP (Game|GetGameInstance)))
  (return (Variables|/Game/Blueprints/FirebrosGameInstance_BP.FirebrosGameInstance_BP_C|GetLocalPlayerName _asfirebros_game_instance_bp)))