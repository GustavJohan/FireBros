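; Lobby mannequin actor for the FireFighter game, with a text render that SetName fills with a given name.
; On BeginPlay it applies physical animation drives from a named bone down and simulates physics on the bodies below that bone, so they react physically while pulled toward the animated pose.
; The Ready replication callback looks up top-level widgets and checks the first for validity, but takes no further action.
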(event EventBeginPlay
  (bind _physicalanimation (Variables|Default|GetPhysicalAnimation))
  (bind _body_name (Variables|Default|GetBody%20Name))
  (Class|PhysicalAnimationComponent|SetSkeletalMeshComponent _physicalanimation (Variables|Default|GetSkeletalMesh))
  (Class|PhysicalAnimationComponent|ApplyPhysicalAnimationSettingsBelow _physicalanimation _body_name (Utilities|Struct|MakePhysicalAnimationData true 1e+03 1e+02 1e+03 1e+02) true)
  (Class|SkeletalMeshComponent|SetAllBodiesBelowSimulatePhysics (Variables|Default|GetSkeletalMesh) _body_name true false))

(event Collision|EventActorBeginOverlap
  (params (OtherActor :type Actor%20Object%20Reference)))

(event EventTick
  (params (DeltaSeconds :type Float%20%28single-precision%29)))

(fn ConstructionScript)

(fn SetName
  (params (Name :type Text))
  (Rendering|Components|TextRender|SetText (Variables|Default|GetTextRender) Name))

(fn OnRepReady
  (bind _foundwidgets (Widget|GetAllWidgetsOfClass 0 true))
  (if (Utilities|IsValid (Utilities|Array|Get(acopy) _foundwidgets))
    _))