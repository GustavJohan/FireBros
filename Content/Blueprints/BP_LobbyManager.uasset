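; BP_LobbyManager handles the player names shown on lobby mannequins, looked up per controller in the PlayerManequins map.
; Setnewname renames one controller's mannequin, while RefreshControllernames reapplies each BP_UIPlayerController's PlayerName.
; SetPlayerName only collects mannequins into an array, which UpdateLobbynames pairs by index with Names through SetNameMulticast.
; The map is not populated here, and the logic that appends to Names and prunes invalid entries is disconnected.
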(event Custom|SetNameMulticast
  (params (Mannequin :type BP%20Lobby%20Manequin%20Object%20Reference) (Name :type Text))
  (if (Utilities|IsValid Mannequin)
    (Default|SetName Mannequin Name)))

(event Custom|Update%20Lobby%20names
  (for (_array_element _array_index) (Variables|Default|GetMannequin)
    (CallFunction|SetNameMulticast _array_element (Utilities|Array|Get(acopy) (Variables|Default|GetNames) _array_index))))

(event Custom|Set%20new%20name
  (params (Name :type Text) (Controller :type Controller%20Object%20Reference))
  (bind _asbp_lobby_manequin (Utilities|Casting|CastToBP_LobbyManequin (.MannequinActor (Utilities|Struct|BreakPlayerMannequinInformation (.Value (Utilities|Map|Find (Variables|Default|GetPlayerManequins) Controller))))))
  (Default|SetName _asbp_lobby_manequin Name))

(event Custom|Refresh%20Controller%20names
  (bind _keys (Utilities|Map|Keys (Variables|Default|GetPlayerManequins)))
  (for _array_element _keys
    (bind _asbp_uiplayer_controller (Utilities|Casting|CastToBP_UIPlayerController _array_element))
    (bind _asbp_lobby_manequin (Utilities|Casting|CastToBP_LobbyManequin (.MannequinActor (Utilities|Struct|BreakPlayerMannequinInformation (.Value (Utilities|Map|Find (Variables|Default|GetPlayerManequins) _asbp_uiplayer_controller))))))
    (Default|SetName _asbp_lobby_manequin (Variables|/Game/Blueprints/BP_PlayerController.BP_PlayerController_C|GetPlayerName _asbp_uiplayer_controller))))

(event EventSetPlayerName
  (params (relevantPlayer :type Controller%20Object%20Reference))
  (bind _playermanequins (Variables|Default|GetPlayerManequins))
  (bind (_value _returnvalue) (Utilities|Map|Find _playermanequins relevantPlayer))
  (bind _asbp_player_controller (Utilities|Casting|CastToBP_PlayerController relevantPlayer))
  (if _returnvalue
    (bind _asbp_lobby_manequin (Utilities|Casting|CastToBP_LobbyManequin (.MannequinActor (Utilities|Struct|BreakPlayerMannequinInformation _value))))
    (Utilities|Array|Add (Variables|Default|GetMannequin) _asbp_lobby_manequin)))

(fn ConstructionScript)