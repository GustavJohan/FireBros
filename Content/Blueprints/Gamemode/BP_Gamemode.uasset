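; Game mode that sets up the manager actors and places joining players at numbered player starts.
; On BeginPlay it spawns a GameManager, then reuses an existing FireManager_BP or spawns one if none is found, storing references to both.
; Each new player restarts at the start found using PlayerNum as its name, with the counter cycling through four slots.
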(event EventBeginPlay
  (bind _returnvalue (Game|SpawnActorfromClass "/Script/FireBros.GameManager" (Math|Transform|MakeTransform "0, 0, 0") "Undefined" "MultiplyWithRoot" (Game|GetPlayerController 0) 0))
  (Variables|Default|SetGameManager _returnvalue)
  (bind _returnvalue_2 (Actor|GetActorOfClass "/Game/Blueprints/FireManager_BP.FireManager_BP_C"))
  (if (Utilities|IsValid _returnvalue_2)
    (Variables|Default|SetFireManager _returnvalue_2)
    (else
      (bind _returnvalue_3 (Game|SpawnActorfromClass "/Game/Blueprints/FireManager_BP.FireManager_BP_C" (Math|Transform|MakeTransform "0, 0, 0") "Undefined" "MultiplyWithRoot" (Game|GetPlayerController 0) 0))
      (Variables|Default|SetFireManager _returnvalue_3))))

(event EventHandleStartingNewPlayer
  (params (NewPlayer :type Player%20Controller%20Object%20Reference))
  (Class|GameModeBase|RestartPlayeratPlayerStart NewPlayer (Class|GameModeBase|FindPlayerStart 0 (Utilities|String|ToString(Integer) (Variables|Default|GetPlayerNum))))
  (bind _result (Math|Integer|IncrementInt (Variables|Default|GetPlayerNum))
    (:%20%20
      (Variables|Default|SetPlayerNum (Math|Integer|%(Integer) _result 4)))))

(fn ConstructionScript)