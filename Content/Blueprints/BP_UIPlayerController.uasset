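; BP_UIPlayerController is a player controller for UI screens that passes player names to the lobby manager.
; On BeginPlay it sets UI-only input and calls SetLocalName, whose body is not in this file.
; SetNewNametoServer waits briefly, finds BP_LobbyManager and hands it the name along with this controller, printing an error if no manager is found.
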(event EventBeginPlay
  (Input|SetInputModeUIOnly self 0 "DoNotLock" false)
  (CallFunction|SetLocalName))

(event EventTick
  (params (DeltaSeconds :type Float%20%28single-precision%29))
  (|CallParentFunction DeltaSeconds) ; This node is disabled and will not be called.\nDrag off pins to build functionality.
)

(event EventSetNewNametoServer
  (params (Name :type Text))
  (Utilities|FlowControl|Delay 0.2)
  (bind _returnvalue (Actor|GetActorOfClass "/Game/Blueprints/Test/BP_LobbyManager.BP_LobbyManager_C"))
  (if (Utilities|IsValid _returnvalue)
    (Default|SetNewName _returnvalue Name self)
    (else
      (Development|PrintString "Lobby manager not found" true true "(R=0.000000,G=0.660000,B=1.000000,A=1.000000)" 3e+01))))

(fn ConstructionScript
  (|CallParentFunction))